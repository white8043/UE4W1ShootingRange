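; Base projectile actor for the shooting range that awards score when its mesh begins overlapping another actor.
; The static mesh's overlap event ignores the projectile's owner and reacts to any other actor.
; It looks up the player by the MainCharacter tag and, if exactly one exists, casts it to BP_BaseCharacter and calls AddScore on its UI.
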(event OnComponentBeginOverlap(StaticMesh)
  (params (OverlappedComponent :type Primitive%20Component%20Object%20Reference) (OtherActor :type Actor%20Object%20Reference) (OtherComp :type Primitive%20Component%20Object%20Reference) (OtherBodyIndex :type Integer) (bFromSweep :type Boolean) (SweepResult :type Hit%20Result%20Structure%20%28by%20ref%29))
  (if (!= OtherActor (Components|GetOwner))
    (bind _outactors (Actor|GetAllActorswithTag "MainCharacter"))
    (if (== (Utilities|Array|Length _outactors) 1)
      (bind _asbp_base_character (Utilities|Casting|CastToBP_BaseCharacter (Utilities|Array|Get(acopy) _outactors)))
      (Default|AddScore (Variables|/Game/ShootingRange/Blueprints/BP_BaseCharacter.BP_BaseCharacter_C|GetUI _asbp_base_character)))))

(event EventBeginPlay)

(event EventTick
  (params (DeltaSeconds :type Float%20%28single-precision%29)))

(fn ConstructionScript)