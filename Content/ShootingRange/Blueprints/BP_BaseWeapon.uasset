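; Base weapon actor for the shooting range that can be picked up, fired and reloaded.
; GetWeapon stores the owning character, disables physics and collision, and derives an aim baseline offset from the Root-to-Sight socket distance.
; With a chambered round, firing plays character and weapon montages, whose notify spawns a muzzle projectile.
; Projectiles head toward the owner's look-at point, or along muzzle forward when absolute yaw reaches 90 degrees.
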(event Custom|MagReloadWeapon
  (Animation|Montage|PlayMontage (Variables|Default|GetSkeletalMesh) "/Game/ShootingRange/Assets/Weapons/AR/AM_AR_Reload_NoCharge.AM_AR_Reload_NoCharge"))

(event EventBeginPlay)

(event Collision|EventActorBeginOverlap
  (params (OtherActor :type Actor%20Object%20Reference)))

(event EventTick
  (params (DeltaSeconds :type Float%20%28single-precision%29)))

(event EventFirePressed
  (bind _skeletalmesh (Variables|Default|GetSkeletalMesh))
  (bind _returnvalue (Transformation|GetSocketTransform _skeletalmesh "Muzzle" "RTS_World"))
  (if (> (Variables|Default|GetRoundsinChamber) 0)
    (Animation|Montage|PlayMontage (Variables|/Script/Engine.Character|GetMesh (Variables|Default|GetOwning%20Character)) "/Game/ShootingRange/Assets/Character/Animation/AM_2HW_ADS_Fire.AM_2HW_ADS_Fire"
      (:then
        (Animation|Montage|PlayMontage (Variables|Default|GetSkeletalMesh) "/Game/ShootingRange/Assets/Weapons/AR/AM_AR_Fire.AM_AR_Fire"
          (:OnNotifyBegin
            (bind _returnvalue_2 (Game|SpawnActorfromClass "/Game/ShootingRange/Blueprints/BP_BaseProjectile.BP_BaseProjectile_C" (Math|Transform|MakeTransform (.location _returnvalue) (.rotation _returnvalue) (* (.scale _returnvalue) 1.0)) "AlwaysSpawn" self 0))
            (Variables|/Script/Engine.MovementComponent|SetVelocity (Variables|/Game/ShootingRange/Blueprints/BP_BaseProjectile.BP_BaseProjectile_C|GetProjectileMovement _returnvalue_2) (* (Math|Vector|SelectVector (Math|Vector|GetForwardVector (Transformation|GetSocketRotation (Variables|Default|GetSkeletalMesh) "Muzzle")) (Math|Vector|Normalize (- (Default|GetActorLookatPoint (Variables|Default|GetOwning%20Character)) (Transformation|GetSocketLocation (Variables|Default|GetSkeletalMesh) "Muzzle"))) (>= (Math|Float|Absolute(Float) (Variables|/Game/ShootingRange/Blueprints/BP_BaseCharacter.BP_BaseCharacter_C|GetYaw (Variables|Default|GetOwning%20Character))) 9e+01)) (Variables|Default|GetMuzzleVelocity)))))))))

(event EventGetWeapon
  (params (OwningCharacter :type BP%20Base%20Character%20Object%20Reference))
  (Variables|Default|SetOwning%20Character OwningCharacter)
  (Physics|SetSimulatePhysics (Variables|Default|GetSkeletalMesh) false)
  (Collision|SetCollisionEnabled (Variables|Default|GetSkeletalMesh) "NoCollision")
  (Variables|Default|SetAimBaselineOffset (- (Class|KismetAnimationLibrary|DistanceBetweenTwoSocketsandMapRange (Variables|Default|GetSkeletalMesh) "Root" "RTS_World" "Sight" "RTS_World" false 0.0 0.0 0.0 0.0) 13.51)))

(fn ConstructionScript)

(fn GetWeaponPanelInfo
  (return self (Variables|Default|GetWeaponType)))